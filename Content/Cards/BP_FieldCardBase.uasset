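; Base class for field cards in a turn-based card game with grid movement, handling clicks, effect hooks and passive effects.
; The controller's first click selects the card and queues creature summon (tribute for rank B+), move or attack on the action stack.
; Clicking again triggers its field/hand effect or flips up set creatures.
; Nested FlipFlops throttle constant-effect updates and passive-effect pruning to every eighth tick; creature logic casts self to child BP_CreatureCardBase.
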(event Custom|NormalSummon
  (bind _controllerplayer (Variables|Default|GetControllerPlayer))
  (switch Utilities|FlowControl|Switch|SwitchonRank (Variables|/Game/Cards/BP_CreatureCardBase.BP_CreatureCardBase_C|GetRank (.AsBP%20Creature%20Card%20Base (Utilities|Casting|CastToBP_CreatureCardBase self)))
    (:NewEnumerator0
      (CallFunction|AddtoActionStack (Utilities|Struct|MakeActionStruct _controllerplayer false "NewEnumerator0" "NewEnumerator0" "NewEnumerator1" "NewEnumerator0" "NewEnumerator0" "NewEnumerator0" false (Utilities|Array|MakeArray "NormalSummon" (select (stale EventClickyClicky Shift) "Shift" "")) "NewEnumerator0" _controllerplayer) :!label _label))
    (:NewEnumerator1
      (goto _label))
    (:NewEnumerator2
      (goto _label))
    (:NewEnumerator3
      (CallFunction|AddtoActionStack (Utilities|Struct|MakeActionStruct _controllerplayer true "NewEnumerator2" "NewEnumerator0" "NewEnumerator2" "NewEnumerator0" "NewEnumerator6" "NewEnumerator0" false (Utilities|Array|MakeArray "TributeForNormalSummon" (select (stale EventClickyClicky Shift) "Shift" "")) "NewEnumerator2" _controllerplayer) :!label _label_2))
    (:NewEnumerator4
      (goto _label_2))
    (:NewEnumerator5
      (goto _label_2))
    (:NewEnumerator6
      (goto _label_2))))

(event Custom|Attacked
  (params (AttackingCreature :type BP%20Creature%20Card%20Base%20Object%20Reference))
  (Default|EffectAttack AttackingCreature)
  (CallFunction|EffectAttacked))

(event Custom|TakeDamage
  (params (Damage :type Integer)))

(event Custom|CheckIfPassiveEffectsAreStillValid
  (for _array_element (Variables|Default|GetPassiveEffects)
    (if (or (not (Utilities|IsValid (.EffectCauser (Utilities|Struct|BreakPassiveEffectStruct _array_element)))) (== (.TurnsRemaining (Utilities|Struct|BreakPassiveEffectStruct _array_element)) 0))
      (Utilities|Array|RemoveItem (Variables|Default|GetPassiveEffects) _array_element))))

(event Custom|Move
  (bind _controllerplayer (Variables|Default|GetControllerPlayer))
  (bind _green (CallFunction|GetCreatureMovementAttackArea false false))
  (CallFunction|AddtoActionStack (Utilities|Struct|MakeActionStruct _controllerplayer "NewEnumerator0" "NewEnumerator0" _green false (Utilities|Array|MakeArray "Move" "UseSuppliedCoords") "NewEnumerator0" _controllerplayer)))

(event Custom|FieldTick
  (CallFunction|EffectConstant)
  (CallFunction|CheckifPassiveEffectsAreStillValid))

(event Custom|Attack
  (bind _controllerplayer (Variables|Default|GetControllerPlayer))
  (bind _red (CallFunction|GetCreatureMovementAttackArea true true))
  (CallFunction|AddtoActionStack (Utilities|Struct|MakeActionStruct _controllerplayer (not _controllerplayer) "NewEnumerator7" "NewEnumerator0" _red false (Utilities|Array|MakeArray "Attack" "UseSuppliedCoords") "NewEnumerator2" _controllerplayer)))

(event EventClickyClicky
  (params (P1 :type Boolean) (Shift :type Boolean))
  (|CallParentFunction P1 Shift)
  (if (CallFunction|IsMyTurn)
    (if (Math|Boolean|Equal(Boolean) (Variables|Default|GetControllerPlayer) P1)
      (if (Default|CanExecuteAction (CallFunction|GetGameBoard))
        (switch Utilities|FlowControl|Switch|SwitchonPosition (Variables|Default|GetPosition)
          (:NewEnumerator0
            (if (== (CallFunction|GetActionReceiverCard) self)
              (bind _asbp_creature_card_base (Utilities|Casting|CastToBP_CreatureCardBase self)
                (:then
                  (if (Variables|/Game/Cards/BP_CreatureCardBase.BP_CreatureCardBase_C|GetSet _asbp_creature_card_base)
                    (if (Variables|/Game/Cards/BP_CreatureCardBase.BP_CreatureCardBase_C|GetCanFlipUp _asbp_creature_card_base)
                      (Default|FlipUp _asbp_creature_card_base true)
                      (else
                        (CallFunction|ClearActionStack true)))
                    (else
                      (bind _canactivate (CallFunction|EffectField? :!label _label))
                      (if _canactivate
                        (CallFunction|EffectField)
                        (else
                          (CallFunction|ClearActionStack true))))))
                (:CastFailed
                  (goto _label)))
              (else
                (CallFunction|SetReceiver Shift)
                (bind _asbp_creature_card_base_2 (Utilities|Casting|CastToBP_CreatureCardBase self))
                (if (not (Variables|/Game/Cards/BP_CreatureCardBase.BP_CreatureCardBase_C|GetSet _asbp_creature_card_base_2))
                  (if (>= (Variables|/Game/Cards/BP_CreatureCardBase.BP_CreatureCardBase_C|GetActionPoints _asbp_creature_card_base_2) 3)
                    (if (and (Utilities|Enum|NotEqual(Enum) (Variables|/Game/Cards/BP_CreatureCardBase.BP_CreatureCardBase_C|GetMovementType _asbp_creature_card_base_2) "NewEnumerator0") (> (Variables|/Game/Cards/BP_CreatureCardBase.BP_CreatureCardBase_C|GetMovementDistance _asbp_creature_card_base_2) 0))
                      (CallFunction|Move))
                    (if (and (Utilities|Enum|NotEqual(Enum) (Variables|/Game/Cards/BP_CreatureCardBase.BP_CreatureCardBase_C|GetAttackType _asbp_creature_card_base_2) "NewEnumerator0") (> (Variables|/Game/Cards/BP_CreatureCardBase.BP_CreatureCardBase_C|GetAttackDistance _asbp_creature_card_base_2) 0))
                      (CallFunction|Attack)))))))
          (:NewEnumerator1
            (if (== (CallFunction|GetActionReceiverCard) self)
              (bind _canactivate_2 (CallFunction|EffectHand?))
              (if _canactivate_2
                (CallFunction|EffectHand)
                (else
                  (CallFunction|ClearActionStack true)))
              (else
                (CallFunction|SetReceiver Shift)
                (bind _asbp_creature_card_base_3 (Utilities|Casting|CastToBP_CreatureCardBase self))
                (if (Utilities|Enum|Equal(Enum) (Variables|/Game/Cards/BP_CreatureCardBase.BP_CreatureCardBase_C|GetSummoningConditions _asbp_creature_card_base_3) "NewEnumerator0")
                  (if (> (Variables|/Game/GameBoardActor.GameBoardActor_C|GetSummons (CallFunction|GetGameBoard)) 0)
                    (CallFunction|NormalSummon)))))))))))

(event EventTick
  (params (DeltaSeconds :type Float%20%28single-precision%29))
  (|CallParentFunction 0.0)
  (Utilities|FlowControl|FlipFlop
    (:A
      (Utilities|FlowControl|FlipFlop
        (:A
          (Utilities|FlowControl|FlipFlop
            (:A
              (CallFunction|FieldTick))))))))

(event EventBeginPlay
  (bind _health0 (Variables|Default|GetHealth0))
  (|CallParentFunction)
  (Variables|Default|SetControllerPlayer (Variables|Default|GetOwnerPlayer))
  (Variables|Default|SetHealth _health0)
  (Variables|Default|SetHealthMax _health0))

(fn ConstructionScript
  (|CallParentFunction))

(fn NextTurn
  (params (P1 :type Boolean))
  (if (Math|Boolean|Equal(Boolean) P1 (Variables|Default|GetControllerPlayer))
    (CallFunction|EffectPlayerTurn)
    (CallFunction|EffectEveryTurn)
    (else
      (CallFunction|EffectOpponentTurn))))

(fn IsMyTurn
  (return (Math|Boolean|Equal(Boolean) (Variables|/Game/GameBoardActor.GameBoardActor_C|GetP1Turn (CallFunction|GetGameBoard)) (Variables|Default|GetControllerPlayer))))

(fn GetCreatureMovementAttackArea
  (params (CheckCollisionGreen :type Boolean) (CheckCollisionRed :type Boolean))
  (bind _array (Utilities|Array|MakeArray))
  (bind _asbp_creature_card_base (Utilities|Casting|CastToBP_CreatureCardBase self)
    (:then
      (bind _green (CallFunction|GetWaterMarkMk2 _asbp_creature_card_base false CheckCollisionGreen false))
      (bind _red (CallFunction|GetWaterMarkMk2 _asbp_creature_card_base false CheckCollisionRed false))
      (for _array_element _green
        (Utilities|Array|AddUnique (LocalVariables|GetG) _array_element))
      (for _array_element_2 _red
        (Utilities|Array|AddUnique (LocalVariables|GetR) _array_element_2))
      (return (LocalVariables|GetG) (LocalVariables|GetR)))
    (:CastFailed
      (return _array _array))))

(fn AddPassiveEffect
  (params (Effect :type Passive%20Effect%20Struct%20Structure))
  (bind (_effect _effectcauser) (Utilities|Struct|BreakPassiveEffectStruct Effect))
  (bind _passiveeffects (Variables|Default|GetPassiveEffects))
  (for _array_element _passiveeffects
    (if (and (Utilities|Enum|Equal(Enum) (.Effect (Utilities|Struct|BreakPassiveEffectStruct _array_element)) _effect) (== (.EffectCauser (Utilities|Struct|BreakPassiveEffectStruct _array_element)) _effectcauser))
      (return false)))
  (Utilities|Array|AddUnique _passiveeffects Effect)
  (return true))

(fn PassiveEffectsContains
  (params (Effect :type String))
  (for _array_element (Variables|Default|GetPassiveEffects)
    (if (Utilities|Enum|Equal(Enum) Effect (.Effect (Utilities|Struct|BreakPassiveEffectStruct _array_element)))
      (return true)))
  (return false))