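; BP_CardBase is the base actor for cards in the Convergence card game, providing overridable hooks for clicks, received targets and zone-specific effects.
; It initializes its card widget with itself and fills the player's mouseover widget on hover.
; Action stack, receiver selection, destruction, draw and tax requests forward to the player controller.
; Received actions dispatch by target type (none, coordinate or card), and mesh materials highlight the active receiver.
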(event OnBeginCursorOver(Widget)
  (params (TouchedComponent :type Primitive%20Component%20Object%20Reference))
  (bind _asplayer_character_convergence (Utilities|Casting|CastToPlayerCharacter_Convergence (Pawn|GetControlledPawn (Game|GetPlayerController 0))))
  (bind _ascard_widget_mouseover (Utilities|Casting|CastToCardWidgetMouseover (UserInterface|GetUserWidgetObject (Variables|/Game/PlayerCharacter_Convergence.PlayerCharacter_Convergence_C|GetMouseoverWidget _asplayer_character_convergence))))
  (Variables|/Game/Cards/CardWidget/CardWidget.CardWidget_C|SetCard _ascard_widget_mouseover self)
  (Default|Init _ascard_widget_mouseover))

(event Custom|ClickyClicky
  (params (P1 :type Boolean) (Shift :type Boolean)))

(event Custom|AddToActionStack
  (params (Action :type Action%20Struct%20Structure))
  (bind _asplayer_controller_convergence (Utilities|Casting|CastToPlayerController_Convergence (Game|GetPlayerController 0)))
  (Default|AddtoActionStack _asplayer_controller_convergence Action))

(event Custom|ClearActionStack
  (params (ResetReceiver :type Boolean) (Override :type Boolean))
  (Default|ClearActionStack (.AsPlayer%20Controller%20Convergence (Utilities|Casting|CastToPlayerController_Convergence (Game|GetPlayerController 0))) ResetReceiver Override))

(event Custom|BecomeReceive
  (params (Shift :type Boolean))
  (Rendering|Material|SetMaterial (Variables|Default|GetStaticMesh1) 0 (select Shift "/Game/Mats/CardSelectedMatShift.CardSelectedMatShift" "/Game/Mats/CardSelectedMat.CardSelectedMat")))

(event Custom|EndReceive
  (Rendering|Material|SetMaterial (Variables|Components|GetStaticMesh) 0 "/Game/Mats/Black.Black")
  (Rendering|Material|SetMaterial (Variables|Default|GetStaticMesh1) 0 "/Game/Mats/NULL.NULL"))

(event Custom|ReceiveAction
  (params (ReceiveType :type ActionReceiveType%20Enum :default "NewEnumerator1") (Coord :type Coordinate%20Structure) (Card :type BP%20Card%20Base%20Object%20Reference) (SpecialInstructions :type Array%20of%20Strings))
  (switch Utilities|FlowControl|Switch|SwitchonActionReceiveType ReceiveType
    (:NewEnumerator1
      (CallFunction|ReceiveNone SpecialInstructions))
    (:NewEnumerator0
      (CallFunction|ReceiveCoord Coord SpecialInstructions))
    (:NewEnumerator2
      (CallFunction|ReceiveCard Card SpecialInstructions))))

(event Custom|SetReceiver
  (params (Shift :type Boolean))
  (Default|SetReceiver (.AsPlayer%20Controller%20Convergence (Utilities|Casting|CastToPlayerController_Convergence (Game|GetPlayerController 0))) self Shift))

(event Custom|DestroyCard
  (params (DeathType :type DeathType%20Enum :default "NewEnumerator0") (DeathCauser :type BP%20Card%20Base%20Object%20Reference) (NoDeathEffect :type Boolean))
  (Default|DestroyCard (.AsPlayer%20Controller%20Convergence (Utilities|Casting|CastToPlayerController_Convergence (Game|GetPlayerController 0))) self DeathType DeathCauser NoDeathEffect))

(event Custom|ReceiveCoord
  (params (Coord :type Coordinate%20Structure) (SpecialInstructions :type Array%20of%20Strings)))

(event Custom|ReceiveCard
  (params (Card :type BP%20Card%20Base%20Object%20Reference) (SpecialInstructions :type Array%20of%20Strings)))

(event Custom|ReceiveNone
  (params (SpecialInstructions :type Array%20of%20Strings)))

(event MouseInput|EventActorOnClicked
  (params (ButtonPressed :type Key%20Structure))
  (if (== ButtonPressed "LeftMouseButton")
    _))

(event EventBeginPlay
  (bind _ascard_widget (Utilities|Casting|CastToCardWidget (UserInterface|GetUserWidgetObject (Variables|Default|GetWidget))))
  (Variables|/Game/Cards/CardWidget/CardWidget.CardWidget_C|SetCard _ascard_widget self)
  (Default|Init _ascard_widget))

(event Custom|Draw
  (params (Amount :type Integer) (SelfDraw :type Boolean))
  (bind _ownerplayer (Variables|Default|GetOwnerPlayer))
  (Default|Draw (CallFunction|GetPlayerController) (select SelfDraw _ownerplayer (not _ownerplayer)) Amount))

(event Custom|Tax
  (params (Amount :type Integer))
  (bind _asplayer_controller_convergence (CallFunction|GetPlayerController))
  (bind _asbp_field_card_base (Utilities|Casting|CastToBP_FieldCardBase self)
    (:then
      (Default|Tax _asplayer_controller_convergence (Variables|/Game/Cards/BP_FieldCardBase.BP_FieldCardBase_C|GetControllerPlayer _asbp_field_card_base) Amount))
    (:CastFailed
      (Default|Tax _asplayer_controller_convergence (Variables|Default|GetOwnerPlayer) Amount))))

(fn ConstructionScript)

(fn EffectField?
  (return false))

(fn EffectGraveyard?
  (return false))

(fn EffectHand?
  (return false))