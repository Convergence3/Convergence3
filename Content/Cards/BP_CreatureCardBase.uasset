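; Base class for creature cards in a grid-based card battler, handling summoning, rank-based tributes, movement, attacks, damage and per-turn action points.
; Action-stack instruction strings select each action, with most game-state changes routed through the player controller.
; Attack hooks spread passive effects to targets or adjacent cards using condition filters.
; Scoring functions rate card and battle value from weighted stats, passives and board position; negative battle value is stubbed at zero.
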(event Custom|FlipUp
  (params (UseEffect :type Boolean))
  (Variables|Default|SetSet false)
  (Variables|Default|SetCanFlipUp false)
  (if UseEffect
    (CallFunction|EffectFlip))
  (CallFunction|EffectSummon))

(event Custom|LoseActionPoints
  (params (Amount :type Integer))
  (Default|LoseActionPoints (CallFunction|GetPlayerController) self Amount))

(event Custom|LoseActionPoints_Internal
  (params (Amount :type Integer))
  (Variables|Default|SetActionPoints (- (Variables|Default|GetActionPoints) Amount)))

(event EventEndReceive
  (|CallParentFunction)
  (Utilities|Array|Clear (Variables|Default|GetSelectedCreatures)))

(event EventEffectAttack
  (params (Attacked :type BP%20Field%20Card%20Base%20Object%20Reference))
  (bind _controllerplayer (Variables|Default|GetControllerPlayer))
  (for _array_element (Variables|Default|GetApplyPassiveEffects)
    (if (or (Utilities|Enum|Equal(Enum) (.SpreadTiming (Utilities|Struct|BreakApplyPassiveEffectStruct _array_element)) "Attack") (Utilities|Enum|Equal(Enum) (.SpreadTiming (Utilities|Struct|BreakApplyPassiveEffectStruct _array_element)) "Battle"))
      (if (Utilities|Enum|Equal(Enum) (.SpreadType (Utilities|Struct|BreakApplyPassiveEffectStruct _array_element)) "Target")
        (Utilities|IsValid Attacked
          (:Is%20Valid
            (bind _asbp_creature_card_base (Utilities|Casting|CastToBP_CreatureCardBase Attacked)
              (:then
                (bind _match_ (CallFunction|MatchesConditions _asbp_creature_card_base (.CreatureCriteriaoptional (Utilities|Struct|BreakApplyPassiveEffectStruct _array_element))))
                (if _match_
                  (Default|AddPassiveEffect Attacked (Utilities|Struct|MakePassiveEffectStruct (.Effect (Utilities|Struct|BreakApplyPassiveEffectStruct _array_element)) self (.TurnsRemainingForEffect (Utilities|Struct|BreakApplyPassiveEffectStruct _array_element)) (.Optionalnumber (Utilities|Struct|BreakApplyPassiveEffectStruct _array_element)) (.Optionalnumber2 (Utilities|Struct|BreakApplyPassiveEffectStruct _array_element)) false false (.SpecialInstruction (Utilities|Struct|BreakApplyPassiveEffectStruct _array_element))) :!label _label)))
              (:CastFailed
                (goto _label)))))
        (elif (Math|Boolean|ORBoolean (Utilities|Enum|Equal(Enum) (.SpreadType (Utilities|Struct|BreakApplyPassiveEffectStruct _array_element)) "Curse") (Utilities|Enum|Equal(Enum) (.SpreadType (Utilities|Struct|BreakApplyPassiveEffectStruct _array_element)) "Aura") (Utilities|Enum|Equal(Enum) (.SpreadType (Utilities|Struct|BreakApplyPassiveEffectStruct _array_element)) "Adjacent"))
          (Utilities|IsValid Attacked
            (:Is%20Valid
              (bind _cards (CallFunction|GetAdjacentFieldCards (Variables|Default|GetCoord) "NewEnumerator2"))
              (for _array_element_2 _cards
                (switch string (.SpreadType (Utilities|Struct|BreakApplyPassiveEffectStruct _array_element))
                  (:Curse
                    (if (Math|Boolean|NotEqual(Boolean) (Variables|/Game/Cards/BP_FieldCardBase.BP_FieldCardBase_C|GetControllerPlayer _array_element_2) _controllerplayer)
                      (bind _asbp_creature_card_base_2 (Utilities|Casting|CastToBP_CreatureCardBase _array_element_2 :!label _label_2)
                        (:then
                          (bind _match__2 (CallFunction|MatchesConditions _asbp_creature_card_base_2 (.CreatureCriteriaoptional (Utilities|Struct|BreakApplyPassiveEffectStruct _array_element))))
                          (if _match__2
                            (Default|AddPassiveEffect _array_element_2 (Utilities|Struct|MakePassiveEffectStruct (.Effect (Utilities|Struct|BreakApplyPassiveEffectStruct _array_element)) self (.TurnsRemainingForEffect (Utilities|Struct|BreakApplyPassiveEffectStruct _array_element)) (.Optionalnumber (Utilities|Struct|BreakApplyPassiveEffectStruct _array_element)) (.Optionalnumber2 (Utilities|Struct|BreakApplyPassiveEffectStruct _array_element)) false false (.SpecialInstruction (Utilities|Struct|BreakApplyPassiveEffectStruct _array_element))) :!label _label_3)))
                        (:CastFailed
                          (goto _label_3)))))
                  (:Aura
                    (if (Math|Boolean|Equal(Boolean) (Variables|/Game/Cards/BP_FieldCardBase.BP_FieldCardBase_C|GetControllerPlayer _array_element_2) _controllerplayer)
                      (goto _label_2)))
                  (:Adjacent
                    (goto _label_2)))))))))))

(event EventEffectAttacked
  (params (Attacker :type BP%20Creature%20Card%20Base%20Object%20Reference))
  (bind _controllerplayer (Variables|Default|GetControllerPlayer))
  (for _array_element (Variables|Default|GetApplyPassiveEffects)
    (if (or (Utilities|Enum|Equal(Enum) (.SpreadTiming (Utilities|Struct|BreakApplyPassiveEffectStruct _array_element)) "Attacked") (Utilities|Enum|Equal(Enum) (.SpreadTiming (Utilities|Struct|BreakApplyPassiveEffectStruct _array_element)) "Battle"))
      (if (Utilities|Enum|Equal(Enum) (.SpreadType (Utilities|Struct|BreakApplyPassiveEffectStruct _array_element)) "Target")
        (bind _match_ (CallFunction|MatchesConditions Attacker (.CreatureCriteriaoptional (Utilities|Struct|BreakApplyPassiveEffectStruct _array_element))))
        (if _match_
          (Default|AddPassiveEffect Attacker (Utilities|Struct|MakePassiveEffectStruct (.Effect (Utilities|Struct|BreakApplyPassiveEffectStruct _array_element)) self (.TurnsRemainingForEffect (Utilities|Struct|BreakApplyPassiveEffectStruct _array_element)) (.Optionalnumber (Utilities|Struct|BreakApplyPassiveEffectStruct _array_element)) (.Optionalnumber2 (Utilities|Struct|BreakApplyPassiveEffectStruct _array_element)) false false (.SpecialInstruction (Utilities|Struct|BreakApplyPassiveEffectStruct _array_element)))))
        (elif (Math|Boolean|ORBoolean (Utilities|Enum|Equal(Enum) (.SpreadType (Utilities|Struct|BreakApplyPassiveEffectStruct _array_element)) "Curse") (Utilities|Enum|Equal(Enum) (.SpreadType (Utilities|Struct|BreakApplyPassiveEffectStruct _array_element)) "Aura") (Utilities|Enum|Equal(Enum) (.SpreadType (Utilities|Struct|BreakApplyPassiveEffectStruct _array_element)) "Adjacent"))
          (bind _cards (CallFunction|GetAdjacentFieldCards (Variables|Default|GetCoord) "NewEnumerator2"))
          (for _array_element_2 _cards
            (switch string (.SpreadType (Utilities|Struct|BreakApplyPassiveEffectStruct _array_element))
              (:Curse
                (if (Math|Boolean|NotEqual(Boolean) (Variables|/Game/Cards/BP_FieldCardBase.BP_FieldCardBase_C|GetControllerPlayer _array_element_2) _controllerplayer)
                  (bind _asbp_creature_card_base (Utilities|Casting|CastToBP_CreatureCardBase _array_element_2 :!label _label)
                    (:then
                      (bind _match__2 (CallFunction|MatchesConditions _asbp_creature_card_base (.CreatureCriteriaoptional (Utilities|Struct|BreakApplyPassiveEffectStruct _array_element))))
                      (if _match__2
                        (Default|AddPassiveEffect _array_element_2 (Utilities|Struct|MakePassiveEffectStruct (.Effect (Utilities|Struct|BreakApplyPassiveEffectStruct _array_element)) self (.TurnsRemainingForEffect (Utilities|Struct|BreakApplyPassiveEffectStruct _array_element)) (.Optionalnumber (Utilities|Struct|BreakApplyPassiveEffectStruct _array_element)) (.Optionalnumber2 (Utilities|Struct|BreakApplyPassiveEffectStruct _array_element)) false false (.SpecialInstruction (Utilities|Struct|BreakApplyPassiveEffectStruct _array_element))) :!label _label_2)))
                    (:CastFailed
                      (goto _label_2)))))
              (:Aura
                (if (Math|Boolean|Equal(Boolean) (Variables|/Game/Cards/BP_FieldCardBase.BP_FieldCardBase_C|GetControllerPlayer _array_element_2) _controllerplayer)
                  (goto _label)))
              (:Adjacent
                (goto _label)))))))))

(event EventNone
  (params (SpecialInstructions :type Array%20of%20Strings))
  (bind _passiveeffects (Variables|Default|GetPassiveEffects))
  (bind (_contains _array_element) (CallFunction|PassiveEffectContains "Consume" _passiveeffects))
  (bind (_effect _effectcauser _turnsremaining _number _number2) (Utilities|Struct|BreakPassiveEffectStruct _array_element))
  (if (Utilities|Array|ContainsItem SpecialInstructions "Consume")
    (if _contains
      (CallFunction|Strengthen _number)
      (CallFunction|Fortify _number2 true))))

(event EventNextTurn
  (params (P1 :type Boolean))
  (|CallParentFunction P1)
  (Variables|Default|SetCanFlipUp true)
  (if (CallFunction|IsMyTurn)
    (if (not (Variables|Default|GetSet))
      (if (not (.Contains (CallFunction|PassiveEffectContains "Exhaust" (Variables|Default|GetPassiveEffects))))
        (if (not (.Contains (CallFunction|PassiveEffectContains "Turtled" (Variables|Default|GetPassiveEffects))))
          (Variables|Default|SetActionPoints (Math|Integer|Clamp(Integer) (+ (Variables|Default|GetActionPoints) (Variables|Default|GetActionPointSpeed)) 0 (Variables|Default|GetActionPointCap))))))))

(event EventEffectPostAttack
  (params (Attacked :type BP%20Field%20Card%20Base%20Object%20Reference))
  (bind _passiveeffects (Variables|Default|GetPassiveEffects))
  (bind (_contains _array_element) (CallFunction|PassiveEffectContains "Consume" _passiveeffects))
  (bind (_effect _effectcauser _turnsremaining _number _number2) (Utilities|Struct|BreakPassiveEffectStruct _array_element))
  (Utilities|IsValid Attacked
    (:Is%20Valid
      (if (.Contains (CallFunction|PassiveEffectContains "Assassin" (Variables|Default|GetPassiveEffects)))
        (Default|DestroyCard Attacked "NewEnumerator1" self false)
        (if _contains :!label _label
          (CallFunction|Strengthen _number)
          (CallFunction|Fortify _number2 true))))
    (:Is%20Not%20Valid
      (goto _label))))

(event EventEffectPostAttacked
  (params (Attack :type BP%20Creature%20Card%20Base%20Object%20Reference)))

(event EventCoord
  (params (Coord :type Coordinate%20Structure) (SpecialInstructions :type Array%20of%20Strings))
  (bind _returnvalue (Utilities|Array|ContainsItem SpecialInstructions "Shift"))
  (Utilities|FlowControl|Sequence
    (:then_0
      (if (and (Utilities|Array|ContainsItem SpecialInstructions "NormalSummon") (Utilities|Enum|Equal(Enum) (Variables|Default|GetSummoningConditions) "NewEnumerator0"))
        (Default|SummonCreatureCardtoCoordinate (.AsPlayer%20Controller%20Convergence (Utilities|Casting|CastToPlayerController_Convergence (Game|GetPlayerController 0))) self Coord true _returnvalue)
        (CallFunction|ClearActionStack true true)
        (elif (Utilities|Array|ContainsItem SpecialInstructions "SpecialSummon")
          (Default|SummonCreatureCardtoCoordinate (CallFunction|GetPlayerController) self Coord false _returnvalue)
          (CallFunction|ClearActionStack true true))))
    (:then_1
      (if (Utilities|Array|ContainsItem SpecialInstructions "Move")
        (Default|MoveCard (.AsPlayer%20Controller%20Convergence (Utilities|Casting|CastToPlayerController_Convergence (Game|GetPlayerController 0))) self Coord)
        (CallFunction|ClearActionStack true false)))))

(event EventAttacked
  (params (AttackingCreature :type BP%20Creature%20Card%20Base%20Object%20Reference))
  (bind _asplayer_controller_convergence (CallFunction|GetPlayerController))
  (bind _self self)
  (if (and (Utilities|IsValid AttackingCreature) (Utilities|IsValid self))
    (|CallParentFunction AttackingCreature)
    (Default|AttackCardCreature _asplayer_controller_convergence AttackingCreature _self))
  (Default|AttackFinalResolution _asplayer_controller_convergence AttackingCreature _self))

(event EventTakeDamage
  (params (Damage :type Integer) (DamageCauser :type BP%20Card%20Base%20Object%20Reference))
  (|CallParentFunction Damage DamageCauser)
  (bind _output_get (Variables|Default|SetHealth (Math|Integer|Clamp(Integer) (- (Variables|Default|GetHealth) (- Damage (Variables|Default|GetShieldFromAdvantage))) 0 (Variables|Default|GetHealth))))
  (if (== _output_get 0)
    (CallFunction|DestroyCard "NewEnumerator1" DamageCauser false)))

(event EventCard
  (params (Card :type BP%20Card%20Base%20Object%20Reference) (SpecialInstructions :type Array%20of%20Strings))
  (bind _self self)
  (bind _selectedcreatures (Variables|Default|GetSelectedCreatures))
  (bind _controllerplayer (Variables|Default|GetControllerPlayer))
  (bind _controllerplayer_2 (Variables|Default|GetControllerPlayer))
  (|CallParentFunction Card SpecialInstructions)
  (Utilities|FlowControl|Sequence
    (:then_0
      (if (Utilities|Array|ContainsItem SpecialInstructions "TributeForNormalSummon")
        (Utilities|Array|AddUnique _selectedcreatures (.AsBP%20Creature%20Card%20Base (Utilities|Casting|CastToBP_CreatureCardBase Card)))
        (if (== (Utilities|Array|Length _selectedcreatures) (Utilities|Select :Index (Variables|Default|GetRank) :NewEnumerator0 0 :NewEnumerator1 0 :NewEnumerator2 0 :NewEnumerator3 1 :NewEnumerator4 2 :NewEnumerator5 3 :NewEnumerator6 3))
          (for _array_element (Variables|Default|GetSelectedCreatures)
            (Default|DestroyCard _array_element "NewEnumerator0" 0 false))
          (CallFunction|ClearActionStack false false)
          (CallFunction|AddtoActionStack (Utilities|Struct|MakeActionStruct _controllerplayer "NewEnumerator0" "NewEnumerator0" "NewEnumerator0" "NewEnumerator1" "NewEnumerator0" "NewEnumerator2" true (Utilities|Array|MakeArray "NormalSummon" (select (Utilities|Array|ContainsItem SpecialInstructions "Shift") "Shift" "")) "NewEnumerator0" _controllerplayer)))))
    (:then_1
      (if (Utilities|Array|ContainsItem SpecialInstructions "Attack")
        (if (Utilities|Array|ContainsItem SpecialInstructions "AttackPlayer")
          (if (== (.X (Utilities|Struct|BreakCoordinate (Variables|Default|GetCoord))) (select _controllerplayer_2 0 6))
            (if (not (.Contains (CallFunction|PassiveEffectContains "Numb" (Variables|Default|GetPassiveEffects))))
              (if (>= (Variables|Default|GetActionPoints) 3)
                (CallFunction|BurnPlayer (Variables|Default|GetAttackDynamic) (not _controllerplayer_2))
                (CallFunction|LoseActionPoints 3)
                (CallFunction|ClearActionStack true false))))
          (else
            (bind _asbp_field_card_base (Utilities|Casting|CastToBP_FieldCardBase Card))
            (Default|Attacked _asbp_field_card_base _self)
            (Default|DecreaseCardActionPoints (CallFunction|GetPlayerController) _self 3)
            (CallFunction|ClearActionStack true false)))))))

(event EventBeginPlay
  (|CallParentFunction)
  (Variables|Default|SetAttribute (Variables|Default|GetAttribute0))
  (Variables|Default|SetMoralAttribute (Variables|Default|GetMoralAttribute0))
  (Variables|Default|SetMovementDistance (Math|Integer|Clamp(Integer) (Variables|Default|GetMovementDistance0) 0 3))
  (Variables|Default|SetAttackDistance (Math|Integer|Clamp(Integer) (Variables|Default|GetAttackDistance0) 0 3))
  (Variables|Default|SetActionPointCap (Variables|Default|GetActionPointCap0))
  (Variables|Default|SetActionPointSpeed (Variables|Default|GetActionPointSpeed0))
  (Variables|Default|SetActionPoints (Variables|Default|GetInitialActionPoints))
  (Variables|Default|SetAttackDynamic (Variables|Default|GetAttack0)))

(event Custom|Strengthen
  (params (Amount :type Integer))
  (Default|GainAttack (CallFunction|GetPlayerController) self Amount))

(event Custom|Strengthen_Internal
  (params (Amount :type Integer))
  (Variables|Default|SetAttackDynamic (Math|Integer|Clamp(Integer) (+ (Variables|Default|GetAttackDynamic) Amount) 0 420)))

(event Custom|Weaken
  (params (Amount :type Integer))
  (CallFunction|Strengthen (* Amount -1)))

(event Custom|Refresh
  (bind _actionreceivecard (CallFunction|GetActionReceiverCard))
  (bind _asbp_creature_card_base (Utilities|Casting|CastToBP_CreatureCardBase _actionreceivecard))
  (CallFunction|Spawn (Utilities|GetClass self) (Variables|Default|GetControllerPlayer) true false false)
  (Default|SummonCreatureCardtoCoordinate (CallFunction|GetPlayerController) _asbp_creature_card_base (Variables|Default|GetCoord) false false)
  (for _array_element (Variables|Default|GetEquipment)
    (Default|Equip _array_element _asbp_creature_card_base))
  (Actor|DestroyActor))

(event Custom|Turtle
  (params (Turtle :type Boolean))
  (Default|Turtle (CallFunction|GetPlayerController) self Turtle))

(fn ConstructionScript
  (|CallParentFunction))

(fn EffectField?
  (return false))

(fn MatchesConditions
  (params (Conditions :type Creature%20Criteria%20Structure))
  (bind (_attribute _moralattribute _rankmin _rankmax _summoningconditions _minactionpoints _setyesnoboth _ownedbyp1p2both _passivestohave _passivestonothave) (Utilities|Struct|BreakCreatureCriteria Conditions))
  (bind _passiveeffects (Variables|Default|GetPassiveEffects))
  (bind _rank (Variables|Default|GetRank))
  (bind _set (Variables|Default|GetSet))
  (bind _controllerplayer (Variables|Default|GetControllerPlayer))
  (bind _has (CallFunction|HasPassiveEffects _passivestohave _passiveeffects))
  (bind _nohas (CallFunction|DoesntHavePassiveEffects _passivestonothave _passiveeffects))
  (return (Math|Boolean|ANDBoolean (or (Utilities|Enum|Equal(Enum) _attribute (Variables|Default|GetAttribute)) (Utilities|Enum|Equal(Enum) _attribute "NewEnumerator0")) (or (Utilities|Enum|Equal(Enum) _moralattribute (Variables|Default|GetMoralAttribute)) (Utilities|Enum|Equal(Enum) _moralattribute "NewEnumerator4")) (and (>= _rank _rankmin) (<= _rank _rankmax)) (or (Utilities|Enum|Equal(Enum) _summoningconditions (Variables|Default|GetSummoningConditions)) (Utilities|Enum|Equal(Enum) _summoningconditions "NewEnumerator0")) (>= (Variables|Default|GetActionPoints) _minactionpoints) (Math|Boolean|Equal(Boolean) (Utilities|Select :Index _setyesnoboth :NewEnumerator0 true :NewEnumerator1 false :NewEnumerator2 _set) _set) (Math|Boolean|Equal(Boolean) _controllerplayer (Utilities|Select :Index _ownedbyp1p2both :NewEnumerator0 true :NewEnumerator1 false :NewEnumerator2 _controllerplayer)) _has _nohas)))

(fn IsTurtled
  (return (.Contains (CallFunction|PassiveEffectContains "Turtled" (Variables|Default|GetPassiveEffects)))))

(fn CanTurtle
  (for _array_element (Variables|Default|GetApplyPassiveEffects)
    (if (Utilities|Enum|Equal(Enum) (.Effect (Utilities|Struct|BreakApplyPassiveEffectStruct _array_element)) "CanTurtle")
      (return true)))
  (return false))

(fn GetCardValue
  (bind _coord (Variables|Default|GetCoord))
  (bind _x (Utilities|Struct|BreakCoordinate _coord))
  (return (+ (* (Variables|Default|GetAttackDynamic) (CallFunction|AttackValueMult)) (* (Variables|Default|GetHealth) (CallFunction|HealthValueMult)) (* (Variables|Default|GetAttackDistance) (CallFunction|AttackDistanceMult)) (* (Variables|Default|GetMovementDistance) (CallFunction|MovementDistanceMult)) (* (Variables|Default|GetActionPointCap) (CallFunction|ActionPointsCapMult)) (* (Variables|Default|GetActionPointSpeed) (CallFunction|ActionPointsSpeedMult)) (* (Variables|Default|GetActionPoints) (CallFunction|ActionPointsMult)) (* (Math|Conversions|ToFloat(Boolean) (Variables|Default|GetSet)) (CallFunction|SetMult)) (CallFunction|CalculatePassiveEffectsValue (Variables|Default|GetPassiveEffects)) (CallFunction|CalculateApplyPassiveEffectsValue (Variables|Default|GetApplyPassiveEffects)) (Variables|Default|GetINHERENTVALUE) (CallFunction|FieldXValue (Utilities|Select :Index (Variables|Default|GetPosition) :NewEnumerator0 (select (Variables|Default|GetControllerPlayer) (- 6 _x) _x) :NewEnumerator1 0 :NewEnumerator2 0 :NewEnumerator3 0)))))

(fn CalculatePassiveEffectsValue
  (params (Passives :type Array%20of%20Passive%20Effect%20Struct%20Structures))
  (if (.Contains (CallFunction|PassiveEffectContains "Seal" Passives))
    _
    (else
      (for _array_element Passives
        (LocalVariables|SetR (+ (LocalVariables|GetR) (CallFunction|GetPassiveEffectValue _array_element))))))
  (return (LocalVariables|GetR)))

(fn GetPassiveEffectValue
  (params (Effect :type Passive%20Effect%20Struct%20Structure))
  (bind (_effect _effectcauser _turnsremaining _number _number2) (Utilities|Struct|BreakPassiveEffectStruct Effect))
  (bind _mult (CallFunction|AttackValueMult))
  (bind _mult_2 (CallFunction|HealthValueMult))
  (bind _returnvalue (* _number _mult))
  (bind _returnvalue_2 (* _number2 _mult_2))
  (bind _returnvalue_3 (+ _returnvalue _returnvalue_2))
  (switch string _effect
    (:Default
      _)
    (:Flying
      (return 3.0))
    (:Tunneling
      (return 3.0))
    (:Intangible
      (return 2.0))
    (:Twoplane
      (return 2.0))
    (:Invisible
      (return 5.0))
    (:Assassin
      (return 5.0))
    (:Numb
      (return -5.0))
    (:Trap
      (return -4.0))
    (:Turtled
      (return 4.0))
    (:TrueSight
      (return 3.0))
    (:Daze
      _)
    (:Seal
      _)
    (:Exhaust
      (return (* (* (Variables|Default|GetActionPointSpeed) (CallFunction|ActionPointsSpeedMult)) -1.0)))
    (:Consume
      (return _returnvalue_3))
    (:DoubleEdge
      (return 3.0))
    (:Invert
      (return 0.0))
    (:Amplify
      (return 2.0))
    (:Battery
      (return (* _returnvalue_3 5.0))))
  (return 0.0))

(fn CalculateApplyPassiveEffectsValue
  (params (Passives :type Array%20of%20Apply%20Passive%20Effect%20Struct%20Structures))
  (for _array_element Passives
    (LocalVariables|SetR (+ (LocalVariables|GetR) (CallFunction|GetApplyPassiveEffectValue _array_element))))
  (return (LocalVariables|GetR)))

(fn GetApplyPassiveEffectValue
  (params (Effect :type Apply%20Passive%20Effect%20Struct%20Structure))
  (bind (_spreadtype _spreadtiming _effect _turnsremainingforeffect _optionalnumber _optionalnumber2) (Utilities|Struct|BreakApplyPassiveEffectStruct Effect))
  (switch string _spreadtype
    (:Default
      _)
    (:Curse
      (LocalVariables|SetMult -1.0))
    (:Aura
      (LocalVariables|SetMult 1.0)))
  (return (* (CallFunction|GetPassiveEffectValue (Utilities|Struct|MakePassiveEffectStruct _effect 0 -1 _optionalnumber _optionalnumber2)) 1.5)))

(fn CalculateBattleValue
  (params (Attacker :type BP%20Creature%20Card%20Base%20Object%20Reference))
  (bind _value__a_positive_number_ (CallFunction|CalculateNegativeBattleValue Attacker))
  (if (.Contains (CallFunction|PassiveEffectContains "Invisible" (Variables|Default|GetPassiveEffects)))
    (if (.Contains (CallFunction|PassiveEffectContains "TrueSight" (Variables|/Game/Cards/BP_FieldCardBase.BP_FieldCardBase_C|GetPassiveEffects Attacker)))
      _
      (else
        (return 0.0))))
  (bind _damage (Default|CalcDamageBetweenCreatures (CallFunction|GetGameBoard) Attacker self))
  (if (or (.Contains (CallFunction|PassiveEffectContains "Assassin" (Variables|/Game/Cards/BP_FieldCardBase.BP_FieldCardBase_C|GetPassiveEffects Attacker))) (<= (- (Variables|Default|GetHealth) _damage) 0))
    (return (- (CallFunction|GetCardValue) _value__a_positive_number_))
    (else
      (return (- (* _damage (CallFunction|HealthValueMult)) _value__a_positive_number_)))))

(fn CalculateNegativeBattleValue
  (params (CardA :type BP%20Creature%20Card%20Base%20Object%20Reference))
  (return 0.0))