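; Base Blueprint for building cards, handling how they take damage and get destroyed.
; When attacked, it calls parent logic, then applies the attacking creature's dynamic attack value as damage.
; TakeDamage subtracts damage from Health, clamped between zero and current Health, and destroys the card when Health reaches zero.
; A field-effect check returns false by default.
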(event EventAttacked
  (params (AttackingCreature :type BP%20Creature%20Card%20Base%20Object%20Reference))
  (|CallParentFunction AttackingCreature)
  (CallFunction|TakeDamage (Variables|/Game/Cards/BP_CreatureCardBase.BP_CreatureCardBase_C|GetAttackDynamic AttackingCreature)))

(event EventTakeDamage
  (params (Damage :type Integer))
  (|CallParentFunction Damage)
  (bind _output_get (Variables|Default|SetHealth (Math|Integer|Clamp(Integer) (- (Variables|Default|GetHealth) Damage) 0 (Variables|Default|GetHealth))))
  (if (== _output_get 0)
    (CallFunction|DestroyCard false)))

(fn ConstructionScript
  (|CallParentFunction))

(fn EffectField?
  (return false))