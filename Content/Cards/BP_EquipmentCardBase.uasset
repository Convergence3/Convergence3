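; Base Blueprint for equipment cards that attach to creatures and lend them passive effects.
; Clicking one in hand on the owner's turn toggles a targeting action over matching field creatures, and the selected creature is equipped.
; Equip and Unequip route through the player controller, with internal events doing the work.
; Equipping copies effects to the creature and moves the card out of hand, while unequipping removes those effects and destroys the card.
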(event Custom|Equip_Internal
  (params (Creature :type BP%20Creature%20Card%20Base%20Object%20Reference))
  (bind _output (CallFunction|GetGameBoard))
  (bind _self self)
  (Utilities|Array|AppendArray (Variables|/Game/Cards/BP_FieldCardBase.BP_FieldCardBase_C|GetPassiveEffects Creature) (Variables|Default|GetPassiveEffectsToBeTransfered))
  (Utilities|Array|AppendArray (Variables|/Game/Cards/BP_FieldCardBase.BP_FieldCardBase_C|GetApplyPassiveEffects Creature) (Variables|Default|GetApplyPassiveEffectsToBeTransfered))
  (Utilities|Array|Add (Variables|/Game/Cards/BP_CreatureCardBase.BP_CreatureCardBase_C|GetEquipment Creature) self)
  (Utilities|Array|RemoveItem (Variables|/Game/GameBoardActor.GameBoardActor_C|GetHandP1 _output) _self)
  (Utilities|Array|RemoveItem (Variables|/Game/GameBoardActor.GameBoardActor_C|GetHandP2 _output) _self)
  (Transformation|DetachFromActor _self "KeepRelative" "KeepRelative" "KeepRelative")
  (bind _player (CallFunction|GetPXPlayerCharacter true))
  (bind _player_2 (CallFunction|GetPXPlayerCharacter false))
  (Default|SortHand _player)
  (Default|SortHand _player_2)
  (Transformation|SetActorTransform (Variables|/Game/GameBoardActor.GameBoardActor_C|GetRemovedCardsTransformP1 _output))
  (CallFunction|ClearActionStack true false))

(event Custom|Unequip_Internal
  (params (Creature :type BP%20Creature%20Card%20Base%20Object%20Reference))
  (bind _self self)
  (for _array_element (Variables|Default|GetPassiveEffectsToBeTransfered)
    (Utilities|Array|RemoveItem (Variables|/Game/Cards/BP_FieldCardBase.BP_FieldCardBase_C|GetPassiveEffects Creature) _array_element))
  (for _array_element_2 (Variables|Default|GetApplyPassiveEffectsToBeTransfered)
    (Utilities|Array|RemoveItem (Variables|/Game/Cards/BP_FieldCardBase.BP_FieldCardBase_C|GetApplyPassiveEffects Creature) _array_element_2))
  (Utilities|Array|RemoveItem (Variables|/Game/Cards/BP_CreatureCardBase.BP_CreatureCardBase_C|GetEquipment Creature) _self)
  (CallFunction|DestroyCard "NewEnumerator0" _self true))

(event Custom|Unequip
  (params (Creature :type BP%20Creature%20Card%20Base%20Object%20Reference))
  (Default|Unequip (CallFunction|GetPlayerController) Creature self))

(event Custom|Equip
  (params (Creature :type BP%20Creature%20Card%20Base%20Object%20Reference))
  (Default|Equip (CallFunction|GetPlayerController) Creature self))

(event EventClickyClicky
  (params (P1 :type Boolean) (Shift :type Boolean))
  (bind _ownerplayer (Variables|Default|GetOwnerPlayer))
  (|CallParentFunction P1 Shift)
  (if (Math|Boolean|Equal(Boolean) (Variables|/Game/GameBoardActor.GameBoardActor_C|GetP1Turn (CallFunction|GetGameBoard)) (Variables|Default|GetOwnerPlayer))
    (if (Default|CanExecuteAction (CallFunction|GetGameBoard))
      (switch Utilities|FlowControl|Switch|SwitchonPosition (Variables|Default|GetPosition)
        (:NewEnumerator1
          (if (== (CallFunction|GetActionReceiverCard) self)
            (CallFunction|ClearActionStack true false)
            (else
              (CallFunction|ClearActionStack true false)
              (CallFunction|SetReceiver false)
              (bind _cards (CallFunction|GetCreaturesonFieldMatchingCriteria (Utilities|Struct|MakeCreatureCriteria "NewEnumerator2" (select _ownerplayer "NewEnumerator0" "NewEnumerator1"))))
              (bind _coords (CallFunction|GetCoordsfromFieldCards _cards))
              (CallFunction|AddtoActionStack (Utilities|Struct|MakeActionStruct _ownerplayer "NewEnumerator2" "NewEnumerator2" "NewEnumerator0" _coords false (Utilities|Array|MakeArray "UseSuppliedCoords" "Select") "NewEnumerator2" _ownerplayer)))))))))

(event EventCard
  (params (Card :type BP%20Card%20Base%20Object%20Reference) (SpecialInstructions :type Array%20of%20Strings))
  (|CallParentFunction Card SpecialInstructions)
  (bind _asbp_creature_card_base (Utilities|Casting|CastToBP_CreatureCardBase Card))
  (CallFunction|Equip _asbp_creature_card_base))

(fn ConstructionScript
  (|CallParentFunction))